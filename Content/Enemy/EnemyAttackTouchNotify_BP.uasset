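; An animation notify that applies an enemy's melee damage at a set point in its attack animation.
; When fired, it takes the owning Enemy and reads its chase target, a ThirdPersonCharacter, from the blackboard's ChaseKey.
; If the target lies within the enemy's attack distance, compared with squared distances, it applies the enemy's damage and returns true; otherwise it returns false.
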(fn `Received_Notify`
  (params (MeshComp :type "SkeletalMeshComponent Object Reference") (Animation :type "AnimSequenceBase Object Reference"))
  (returns (ReturnValue :type Boolean))
  (bind _asenemy (cast `/Game/Enemy/Enemy` (`ActorComponent.GetOwner` MeshComp))
    (:`then`
      (bind _asthird_person_character (cast `/Game/ThirdPersonBP/Blueprints/ThirdPersonCharacter` (`BlackboardComponent.GetValueAsObject` (`AIBlueprintHelperLibrary.GetBlackboard` _asenemy) (`self.Chase Key`)))
        (:`then`
          (if (<= (`KismetMathLibrary.Vector_DistanceSquared` (`Actor.K2_GetActorLocation` _asenemy) (`Actor.K2_GetActorLocation` _asthird_person_character)) (`KismetMathLibrary.Square` (`/Game/Enemy/Enemy.DistanceToAttack` _asenemy)))
            (`/Game/Enemy/Enemy.ApplyDamage` _asenemy (`/Game/Enemy/Enemy.damage` _asenemy) _asthird_person_character)
            (return true)
            (else
              _)))
        (:`CastFailed`
          _)))
    (:`CastFailed`
      _))
  (return false))