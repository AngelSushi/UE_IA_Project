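; Pet Blueprint that lets the player's third-person character interact with it while perceived by the pet.
; AI Perception target updates are filtered to ThirdPersonCharacter; a successful sense creates and shows a PetWidget, and a lost one removes it and clears the stored reference.
; The same sensed state is written to the character's CanInteractWithPet flag, with no Tick logic involved.
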(event `self.AIPerception.OnTargetPerceptionUpdated`
  (params (Actor :type "Actor Object Reference") (Stimulus :type "AIStimulus Structure"))
  (bind (_age _expirationage _strength _stimuluslocation _receiverlocation _tag _bsuccessfullysensed) (break `AIStimulus` Stimulus))
  (bind _asthird_person_character (cast `/Game/ThirdPersonBP/Blueprints/ThirdPersonCharacter` Actor))
  (`|ExecutionSequence`
    (:`then_0`
      (if _bsuccessfullysensed
        (bind _returnvalue (`|CreateWidget` "/Game/Widget/PetWidget.PetWidget_C"))
        (`UserWidget.AddToViewport` _returnvalue 0)
        (set `self.lastWidget` _returnvalue)
        (else
          (`Widget.RemoveFromParent` (`self.lastWidget`))
          (set `self.lastWidget` null))))
    (:`then_1`
      (set `/Game/ThirdPersonBP/Blueprints/ThirdPersonCharacter.CanInteractWithPet` _bsuccessfullysensed _asthird_person_character))))

(fn `UserConstructionScript`)